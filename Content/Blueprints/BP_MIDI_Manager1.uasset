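; BP_MIDI_Manager1 is a manager that connects a chosen MIDI input device to MetaSound synth sounds.
; BeginPlay scans devices for the receivable one matching MIDIControllerIndex1, binds its MIDI events, then starts MSS_MonoSynth.
; The event handler prints type, note and velocity, and on Note On creates MSS_Polysynth without playing it or passing the note.
; An MSS_Synth01 chain setting a MIDINote parameter is left unconnected.
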(event Custom|EventOnMidiEvent
  (params (MIDIDeviceController :type MIDI%20Device%20Controller%20Object%20Reference) (Timestamp :type Integer) (EventType :type EMIDIEventType%20Enum :default "Unknown") (Channel :type Integer) (ControlID :type Integer) (Velocity :type Integer) (RawEventType :type Integer))
  (Development|PrintString (Utilities|String|ToString(Text) (Utilities|Text|FormatText "MIDI EVENT TYPE {event} MIDI Note {note} Vélocité {Velocité}" ControlID Velocity (Utilities|String|EnumtoString EventType))))
  (switch Utilities|FlowControl|Switch|SwitchonEMIDIEventType EventType
    (:NoteOn
      (Audio|CreateSound2D "/Game/Metasound/MSS_Polysynth.MSS_Polysynth" 1.0 1.0 0.0 0))))

(event EventBeginPlay
  (bind _outmididevices (Class|MIDIDeviceManager|FindMIDIDevices))
  (for _array_element _outmididevices
    (if (.bCanReceiveFrom (Utilities|Struct|BreakFoundMIDIDevice _array_element))
      (if (== (Variables|Default|GetMIDIControllerIndex1) (.DeviceID (Utilities|Struct|BreakFoundMIDIDevice _array_element)))
        (Development|PrintString (.DeviceName (Utilities|Struct|BreakFoundMIDIDevice _array_element)) true true "(R=0.000000,G=0.660000,B=1.000000,A=1.000000)" 2.9e+02 "MIDI")
        (bind _returnvalue (Class|MIDIDeviceManager|CreateMIDIDeviceController (.DeviceID (Utilities|Struct|BreakFoundMIDIDevice _array_element)) 1024))
        (bind _output_get (Variables|Default|SetNewVar _returnvalue))
        (EventDispatchers|BindEventtoOnMIDIEvent _output_get (EventDispatchers|CreateEvent :!event Custom|EventOnMidiEvent)))))
  (Development|PrintString "BOUCLE TERMINÉE" true true "(R=0.000000,G=0.660000,B=1.000000,A=1.000000)" 2e+01)
  (bind _returnvalue_2 (Audio|CreateSound2D "/Game/Metasound/MSS_MonoSynth.MSS_MonoSynth" 1.0 1.0 0.0 0))
  (Audio|Components|Audio|Play _returnvalue_2 0.0))

(fn ConstructionScript)