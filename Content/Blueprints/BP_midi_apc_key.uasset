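; Actor Blueprint that connects an Akai APC Key 25 MIDI controller for input and output.
; On BeginPlay it filters the connected MIDI devices by the desired name, then opens the first match as input and the second as output, without checking that both exist.
; The input's MIDI event is bound, but the custom event handler is empty and nothing is sent to the output yet.
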(event Custom|CustomEvent
  (params (MIDIDeviceController :type MIDI%20Device%20Controller%20Object%20Reference) (Timestamp :type Integer) (EventType :type EMIDIEventType%20Enum :default "Unknown") (Channel :type Integer) (ControlID :type Integer) (Velocity :type Integer) (RawEventType :type Integer)))

(event EventBeginPlay
  (bind _outmididevices (Class|MIDIDeviceManager|FindMIDIDevices))
  ;[1 1 1] Find desired relevant devices in array
  (for _array_element _outmididevices
    (if (Utilities|Enum|Equal(Enum) (.DeviceName (Utilities|Struct|BreakFoundMIDIDevice _array_element)) (Variables|Default|GetDesired-Device-Name))
      (Utilities|Array|Add (Variables|Default|GetRelevant-Midi-Devices) _array_element)))
  ;[1 1 1] Set incoming Midi Device and bind to change event
  (bind _returnvalue (Class|MIDIDeviceManager|CreateMIDIDeviceController (.DeviceID (Utilities|Struct|BreakFoundMIDIDevice (Utilities|Array|Get(acopy) (Variables|Default|GetRelevant-Midi-Devices)))) 1024))
  (bind _output_get (Variables|Default|SetAPC_KEY25 _returnvalue))
  (EventDispatchers|BindEventtoOnMIDIEvent _output_get (EventDispatchers|CreateEvent :!event Custom|CustomEvent))
  ;[1 1 1] Set outgoing device to send Midi to
  (bind _returnvalue_2 (Class|MIDIDeviceManager|CreateMIDIDeviceOutputController (.DeviceID (Utilities|Struct|BreakFoundMIDIDevice (Utilities|Array|Get(acopy) (Variables|Default|GetRelevant-Midi-Devices) 1)))))
  (Variables|Default|SetOutput-APC_Key25 _returnvalue_2))

(event Collision|EventActorBeginOverlap
  (params (OtherActor :type Actor%20Object%20Reference)))

(event EventTick
  (params (DeltaSeconds :type Float%20%28single-precision%29)))

(fn ConstructionScript)