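; MIDI manager that plays a polyphonic MetaSound synth from a hardware MIDI controller.
; On BeginPlay it opens the input device matching MIDIControllerIndex and binds its MIDI events.
; Note On spawns an MSS_Stereo voice stored by note number, Note Off triggers its release, and Control Change drives Amount on valid voices.
; An earlier monosynth setup with per-knob filter, decay and drive controls remains disconnected.
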(event Custom|EventonMIDI
  (params (MIDIDeviceController :type MIDI%20Device%20Controller%20Object%20Reference) (Timestamp :type Integer) (EventType :type EMIDIEventType%20Enum :default "Unknown") (Channel :type Integer) (ControlID :type Integer) (Velocity :type Integer) (RawEventType :type Integer))
  (bind _returnvalue (Math|Conversions|ToFloat(Integer) ControlID))
  (bind _returnvalue_2 (Math|Float|Truncate _returnvalue))
  ;[0.15 0.15 0.15 0.5] Imprimer à l'écran
  (Development|PrintString (Utilities|String|ToString(Text) (Utilities|Text|FormatText "MIDI EVENT TYPE {event} MIDI note{note} VELOCITE {velocite}" (Utilities|String|EnumtoString EventType) ControlID Velocity)) true true "(R=0.168419,G=1.000000,B=0.247111,A=1.000000)" 2.0 "MIDI")
  (switch Utilities|FlowControl|Switch|SwitchonEMIDIEventType EventType
    (:NoteOff
      (Class|AudioParameterControllerInterface|SetTriggerParameter (Utilities|Array|Get(acopy) (Variables|Default|Getpolyvoices) _returnvalue_2) "Trigger Release"))
    (:NoteOn
      (bind _returnvalue_3 (Audio|CreateSound2D "/Game/Metasound/MSS_Stereo.MSS_Stereo" 1.0 1.0 0.0 0))
      (Utilities|Array|SetArrayElem (Variables|Default|Getpolyvoices) _returnvalue_2 _returnvalue_3 true)
      (Audio|Parameter|SetFloatParameter _returnvalue_3 "MIDI note" _returnvalue :!class /Script/AudioExtensions.AudioParameterControllerInterface)
      (Audio|Components|Audio|Play _returnvalue_3 0.0))
    (:ControlChange
      (switch string (Utilities|String|ToString(Integer) ControlID)
        (:74
          (for _array_element (Variables|Default|Getpolyvoices)
            (Utilities|IsValid _array_element
              (:Is%20Valid
                (Audio|Parameter|SetFloatParameter _array_element "Amount" (/ (Math|Conversions|ToFloat(Integer) Velocity) 127.0) :!class /Script/AudioExtensions.AudioParameterControllerInterface)))))))))

(event EventBeginPlay
  (bind _outmididevices (Class|MIDIDeviceManager|FindMIDIDevices))
  (for _array_element _outmididevices
    (if (.bCanReceiveFrom (Utilities|Struct|BreakFoundMIDIDevice _array_element))
      (if (== (Variables|Default|GetMIDI_controller_index) (.DeviceID (Utilities|Struct|BreakFoundMIDIDevice _array_element)))
        (Development|PrintString (.DeviceName (Utilities|Struct|BreakFoundMIDIDevice _array_element)) true true "(R=0.000000,G=0.660000,B=1.000000,A=1.000000)" 3e+01)
        (bind _returnvalue (Class|MIDIDeviceManager|CreateMIDIDeviceController (.DeviceID (Utilities|Struct|BreakFoundMIDIDevice _array_element)) 1024))
        (bind _output_get (Variables|Default|SetMIDIcontrol _returnvalue))
        (EventDispatchers|BindEventtoOnMIDIEvent _output_get (EventDispatchers|CreateEvent :!event Custom|EventonMIDI)))))
  (Development|PrintString "BOUCLE TERMINÉE" true true "(R=0.000000,G=0.660000,B=1.000000,A=1.000000)" 3e+01))

(fn ConstructionScript)